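; Base enemy Blueprint that registers with BP_GameMode's enemy count, plays a spawn animation, then moves along the world X axis.
; BeginPlay randomizes direction and speed, then a timeline lowers the actor from its spawn point and enables movement when finished.
; Tick applies delta-scaled movement without sweep, but picks the sign from MoveEnabled, leaving MoveDirection unused and movement always using the positive multiplier.
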(event `self.ReceiveBeginPlay`
  (bind _spawnlocation (`self.SpawnLocation`))
  ;[1 1 1] Setup References and Variables
  (bind _asbp_game_mode (cast `/Game/Blueprints/BP_GameMode` (`GameplayStatics.GetGameMode`)))
  (bind _output_get (set `self.BP_GameMode` _asbp_game_mode))
  (`/Game/Blueprints/BP_GameMode.UpdateEnemyCount` _output_get 1)
  (set `self.MoveDirection` (`KismetMathLibrary.RandomBool`))
  (set `self.MovementSpeed` (`KismetMathLibrary.RandomFloatInRange` (`self.MinimumSpeed`) (`self.MaximumSpeed`)))
  (set `self.SpawnLocation` (`self.K2_GetActorLocation`))
  ;[1 1 1] Spawn Animation
  (bind (_direction _speed) (`Timeline|SpawnAnimation`)
    (:`Update`
      (`self.K2_SetActorLocation` (`KismetMathLibrary.VLerp` _spawnlocation (- _spawnlocation (0.0 0.0 120.0)) _speed)))
    (:`Finished`
      (set `self.MoveEnabled` true))))

(event `self.ReceiveTick`
  (params (DeltaSeconds :type "Float (single-precision)"))
  (if (`self.MoveEnabled`)
    (`self.K2_SetActorLocation` (+ (`self.K2_GetActorLocation`) (* (`KismetMathLibrary.MakeVector` (* (`self.MovementSpeed`) (`KismetMathLibrary.SelectFloat` 1.0 -1.0 (`self.MoveEnabled`)))) DeltaSeconds)))))

(fn `UserConstructionScript`)