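; Player Blueprint that plays a timeline-driven move to its start location on spawn, then sets MoveEnabled.
; MoveUp and MoveRight axis inputs feed a shared Movement function that eases vertical and horizontal speeds toward their targets.
; Tick applies those speeds as separate swept X and Z offsets, not scaled by delta time.
; It also turns the mesh's yaw with horizontal speed at a constant interpolation rate.
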(event `self.ReceiveBeginPlay`
  ;[1 1 1] Player Spawn Animation
  (bind _asbp_game_mode (cast `/Game/Blueprints/BP_GameMode` (`GameplayStatics.GetGameMode`)))
  (set `self.BP_GameMode` _asbp_game_mode)
  (bind (_direction _speed) (`Timeline|SpawnAnimation`)
    (:`Update`
      (`self.SpawnToStartLocation` _speed))
    (:`Finished`
      (set `self.MoveEnabled` true))))

(event `InputAxis|MoveUp`
  (params (AxisValue :type "Float (single-precision)"))
  ;[1 1 1] Player Input
  (bind _returndirectionspeed (`self.Movement` (`self.VerticalSpeed`) AxisValue))
  (set `self.VerticalSpeed` _returndirectionspeed))

(event `InputAxis|MoveRight`
  (params (AxisValue :type "Float (single-precision)"))
  ;[1 1 1] Player Input
  (bind _returndirectionspeed (`self.Movement` (`self.HorizontalSpeed`) AxisValue))
  (set `self.HorizontalSpeed` _returndirectionspeed))

(event `self.ReceiveTick`
  (params (DeltaSeconds :type "Float (single-precision)"))
  (bind _playermesh (`self.PlayerMesh`))
  ;[1 1 1] Movement
  (set `self.DeltaSeconds` DeltaSeconds)
  (`self.K2_SetActorLocation` (+ (`self.K2_GetActorLocation`) (`KismetMathLibrary.MakeVector` (`self.HorizontalSpeed`))) true)
  (`self.K2_SetActorLocation` (+ (`self.K2_GetActorLocation`) (`KismetMathLibrary.MakeVector` 0.0 0.0 (`self.VerticalSpeed`))) true)
  (`SceneComponent.K2_SetRelativeRotation` _playermesh (`KismetMathLibrary.RInterpTo_Constant` (`SceneComponent.RelativeRotation` _playermesh) (`KismetMathLibrary.MakeRotator` 0.0 0.0 (+ (* (`self.HorizontalSpeed`) -7.0) (`self.Yaw`))) (`self.DeltaSeconds`) 80.0) false false))

(fn `Movement`
  (params (Speed :type "Float (double-precision)") (Direction :type "Float (double-precision)"))
  (returns (ReturnDirectionSpeed :type "Float (double-precision)"))
  (return (`KismetMathLibrary.FInterpTo` Speed (* (`self.MovementSpeed`) Direction) (`self.DeltaSeconds`) 6.0)))

(fn `UserConstructionScript`)